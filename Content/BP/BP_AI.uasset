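; Civilian AI character that joins the player's group and can be sent into bunkers or habitations.
; On capsule overlap with the player, it registers itself, takes the player's newest civilian position and writes it to the blackboard to start movement.
; Enter targets the building's entry as the Door key, or without a valid building calls StopQueue, which clears InQueue recursively along the NextToEnter chain.
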(event `self.ReceiveBeginPlay`
  (bind _returnvalue (`AIBlueprintHelperLibrary.GetBlackboard` (`AIBlueprintHelperLibrary.GetAIController` self)))
  (`BlackboardComponent.SetValueAsObject` _returnvalue "PosToHave" (`self.Pos`))
  (`BlackboardComponent.SetValueAsBool` _returnvalue "MoveTo" true)
  (`BlackboardComponent.SetValueAsBool` _returnvalue "ToPlayer" true))

(event `self.CapsuleComponent.OnComponentBeginOverlap`
  (params (OverlappedComponent :type "PrimitiveComponent Object Reference") (OtherActor :type "Actor Object Reference") (OtherComp :type "PrimitiveComponent Object Reference") (OtherBodyIndex :type Integer) (bFromSweep :type Boolean) (SweepResult :type "HitResult Structure (by ref)"))
  (bind _returnvalue (`AIBlueprintHelperLibrary.GetBlackboard` null))
  (if (not (`self.InQueue`))
    (bind _asbp_third_person_character (cast `/Game/ThirdPerson/Blueprints/BP_ThirdPersonCharacter` OtherActor))
    (set `self.InQueue` true)
    (`KismetSystemLibrary.PrintString` (`KismetSystemLibrary.GetDisplayName` _asbp_third_person_character))
    (`/Game/ThirdPerson/Blueprints/BP_ThirdPersonCharacter.AddCivilPos` _asbp_third_person_character)
    (`KismetArrayLibrary.Array_Add` (`/Game/ThirdPerson/Blueprints/BP_ThirdPersonCharacter.OwnCivil` _asbp_third_person_character) self)
    (bind _civilspos (`/Game/ThirdPerson/Blueprints/BP_ThirdPersonCharacter.CivilsPos` _asbp_third_person_character))
    (bind _output_get (set `self.Pos` (`|GetArrayItem` _civilspos (`KismetArrayLibrary.Array_LastIndex` _civilspos))))
    (`/Game/ThirdPerson/Blueprints/BP_ThirdPersonCharacter.UpdateCivilGroupText` _asbp_third_person_character)
    (`BlackboardComponent.SetValueAsObject` _returnvalue "PosToHave" _output_get)
    (`BlackboardComponent.SetValueAsBool` _returnvalue "MoveTo" true)
    (`BlackboardComponent.SetValueAsBool` _returnvalue "ToPlayer" true)))

(fn `Enter`
  (bind _building (`self.Building`))
  (bind _returnvalue (`AIBlueprintHelperLibrary.GetBlackboard` (`AIBlueprintHelperLibrary.GetAIController` self)))
  (`/Engine/EditorBlueprintResources/StandardMacros.IsValid` _building
    (:`Is Valid`
      (bind _asbp_bunker (cast `/Game/BP/Building/Bp_Bunker` _building)
        (:`then`
          (`BlackboardComponent.SetValueAsObject` _returnvalue "Door" (`/Game/BP/Building/Bp_Bunker.Entry` _asbp_bunker)))
        (:`CastFailed`
          (bind _asbp_habitation (cast `/Game/BP/Building/BP_Habitation` _building))
          (`BlackboardComponent.SetValueAsObject` _returnvalue "Door" (`/Game/BP/Building/BP_Habitation.Entry` _asbp_habitation))))
      (`BlackboardComponent.SetValueAsBool` _returnvalue "MoveTo" true))
    (:`Is Not Valid`
      (`self.StopQueue`))))

(fn `StopQueue`
  (bind _nexttoenter (`self.NextToEnter`))
  (set `self.InQueue` false)
  (`/Engine/EditorBlueprintResources/StandardMacros.IsValid` _nexttoenter
    (:`Is Valid`
      (`self.StopQueue` _nexttoenter))))

(fn `UserConstructionScript`)