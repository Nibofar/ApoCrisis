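; BP_Ruin is a grid-placed ruin actor that orients itself by its position relative to the grid origin.
; The Construction Script compares the signs and magnitudes of GridX and GridY, then snaps rotation in quarter turns to face outward along the dominant axis.
; A ruin at the origin gets a random one of the four rotations.
; The event graph holds only disabled placeholder events.
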(fn `UserConstructionScript`
  (bind _gridx (`self.GridX`))
  (bind _gridy (`self.GridY`))
  (bind _returnvalue (== _gridy 0))
  (bind _returnvalue_2 (== _gridx 0))
  (bind _returnvalue_3 (> _gridy 0))
  (if (and _returnvalue_2 _returnvalue)
    (switch `int` (`KismetMathLibrary.RandomInteger` 4)
      (:`0`
        (`self.K2_SetActorRotation` (struct) :!label _label))
      (:`1`
        (`self.K2_SetActorRotation` (struct :`Yaw` 90.0) :!label _label_2))
      (:`2`
        (`self.K2_SetActorRotation` (struct :`Yaw` 180.0) :!label _label_3))
      (:`3`
        (`self.K2_SetActorRotation` (struct :`Yaw` 270.0) :!label _label_4)))
    (elif _returnvalue_2
      (if (> _gridy 0)
        (goto _label_2)
        (else
          (goto _label_4)))
      (elif _returnvalue
        (if (> _gridx 0)
          (goto _label)
          (else
            (goto _label_3)))
        (elif (> _gridx 0)
          (if _returnvalue_3
            (if (>= _gridx _gridy)
              (goto _label)
              (else
                (goto _label_2)))
            (elif (> _gridx (* _gridy -1))
              (goto _label)
              (else
                (goto _label_4))))
          (elif _returnvalue_3
            (if (>= (* _gridx -1) _gridy)
              (goto _label_3)
              (else
                (goto _label_2)))
            (elif (> _gridx _gridy)
              (goto _label_4)
              (else
                (goto _label_3)))))))))