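; Map manager that builds a grid-based city and drops meteors on it.
; BeginPlay fills a flat grid-state array, spawns a rounded block of habitations and turns a random one into the bunker.
; The U key adds habitations, using a direction state machine to walk a cursor around the city's edge.
; Every ten seconds, or on M, a meteor spawns above a random habitation cell, marking it and flagging any matching listed habitation.
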(event `self.ReceiveBeginPlay`
  (`self.GenerateGrid`)
  (`self.Spawn Base City`)
  (set `self.PointeurX` -1)
  (set `self.PointeurY` 4))

(event `Key|U`
  (params (Key :type "Key Structure"))
  (:`Pressed`
    (`self.IncreaseCity`)))

(event `Key|M`
  (params (Key :type "Key Structure"))
  (:`Pressed`
    (`self.SpawnMeteor`)))

(event `self.ReceiveTick`
  (params (DeltaSeconds :type "Float (single-precision)"))
  (bind _output_get (set `self.Timer` (+ DeltaSeconds (stale _output_get))))
  (if (> _output_get 10.0)
    (set `self.Timer` 0.0)
    (`self.SpawnMeteor`)))

(fn `GenerateGrid`
  (for _ (range (+ (* (`self.OffsetGrid`) (`self.OffsetGrid`)) 1))
    (`KismetArrayLibrary.Array_Add` (`self.GridData`) "NewEnumerator0")))

(fn `IncreaseCity`
  (locals (Offset :type "Float (double-precision)" :default 1000.0))
  (bind _pointeury (`self.PointeurY`))
  (bind _pointeury_2 (`self.PointeurY`))
  (bind _pointeurx (`self.PointeurX`))
  (bind _pointeury_3 (`self.PointeurY`))
  (bind _pointeurx_2 (`self.PointeurX`))
  (bind _pointeury_4 (`self.PointeurY`))
  (bind _pointeurx_3 (`self.PointeurX`))
  (bind _pointeury_5 (`self.PointeurY`))
  (bind _pointeury_6 (`self.PointeurY`))
  (bind _pointeurx_4 (`self.PointeurX`))
  (bind _offset (`local.Offset`))
  (bind _pointeurx_5 (`self.PointeurX`))
  (bind _returnvalue (+ (`self.PointeurX`) -1))
  (bind _returnvalue_2 (+ (`self.PointeurY`) -1))
  (bind _returnvalue_3 (+ (`self.PointeurX`) 1))
  (bind _returnvalue_4 (+ (`self.PointeurY`) -1))
  (bind _returnvalue_5 (+ (`self.PointeurX`) 1))
  (bind _returnvalue_6 (+ (`self.PointeurY`) 1))
  (bind _returnvalue_7 (+ (`self.PointeurX`) -1))
  (bind _returnvalue_8 (+ (`self.PointeurY`) 1))
  (bind _returnvalue_9 (+ _returnvalue_5 1))
  (`|SpawnActorFromClass` "/Game/BP/Building/BP_Habitation.BP_Habitation_C" (`KismetMathLibrary.MakeTransform` (`KismetMathLibrary.MakeVector` (* _offset _pointeurx_4) (* _offset _pointeury_2) 100.0)) "Undefined" "OverrideRootScale" null _pointeurx_4 _pointeury_2 null)
  (`KismetArrayLibrary.Array_Set` (`self.GridData`) (`self.PosToIndex` _pointeurx_4 _pointeury_2) "NewEnumerator1")
  (switch `/Game/BP/Enum_IncreaseCity` (`self.IncreaseState`)
    (:`NewEnumerator0`
      ;[1 1 1] All Top Right
      (if (not (`self.GetGridState` _returnvalue_3 _returnvalue_4))
        (if (not (`self.GetGridState` _returnvalue_3 (+ _returnvalue_4 -1)))
          (set `self.IncreaseState` "NewEnumerator1"))
        (`/Engine/EditorBlueprintResources/StandardMacros.DecrementInt` (`self.PointeurY`)
          (:`  `
            _)))
      (`/Engine/EditorBlueprintResources/StandardMacros.IncrementInt` (`self.PointeurX`)))
    (:`NewEnumerator1`
      ;[1 1 1] All Bot Right
      (if (not (`self.GetGridState` _returnvalue _returnvalue_2))
        (if (not (`self.GetGridState` (+ _returnvalue -1) _returnvalue_2))
          (set `self.IncreaseState` "NewEnumerator2"))
        (`/Engine/EditorBlueprintResources/StandardMacros.DecrementInt` (`self.PointeurX`)
          (:`  `
            _)))
      (`/Engine/EditorBlueprintResources/StandardMacros.DecrementInt` (`self.PointeurY`)))
    (:`NewEnumerator2`
      ;[1 1 1] All Bot Left
      (if (not (`self.GetGridState` _returnvalue_7 _returnvalue_8))
        (if (not (`self.GetGridState` _returnvalue_7 (+ _returnvalue_8 1)))
          (set `self.IncreaseState` "NewEnumerator3"))
        (`/Engine/EditorBlueprintResources/StandardMacros.IncrementInt` (`self.PointeurY`)
          (:`  `
            _)))
      (`/Engine/EditorBlueprintResources/StandardMacros.DecrementInt` (`self.PointeurX`)))
    (:`NewEnumerator3`
      ;[1 1 1] All Top Left
      (if (`self.GetGridState` _returnvalue_5 _returnvalue_6)
        (if (`self.GetGridState` _returnvalue_9 (+ _returnvalue_6 1))
          (`/Engine/EditorBlueprintResources/StandardMacros.IncrementInt` (`self.PointeurY`) :!label _label)
          (else
            (if (`self.Repeat`)
              (set `self.IncreaseState` "NewEnumerator0")
              (set `self.PointeurY` (+ _pointeury 2))
              (`/Engine/EditorBlueprintResources/StandardMacros.IncrementInt` _pointeurx_5
                (:`  `
                  _))
              (else
                (set `self.IncreaseState` "NewEnumerator4")
                (`/Engine/EditorBlueprintResources/StandardMacros.IncrementInt` _pointeury
                  (:`  `
                    (`/Engine/EditorBlueprintResources/StandardMacros.IncrementInt` _pointeurx_5 :!label _label_2
                      (:`  `
                        (if (`self.GetGridState` _pointeurx_5 _pointeury)
                          (goto _label_2)
                          (else
                            _))))))))
            (set `self.Repeat` (not (`self.Repeat`)))))
        (elif (`self.GetGridState` _returnvalue_9 _returnvalue_6)
          (`/Engine/EditorBlueprintResources/StandardMacros.IncrementInt` (`self.PointeurX`)
            (:`  `
              (goto _label))))))
    (:`NewEnumerator4`
      ;[1 1 1] Diag Top Right
      (if (`self.GetGridState` (+ (`self.PointeurX`) 1) (+ (`self.PointeurY`) -2))
        (`/Engine/EditorBlueprintResources/StandardMacros.IncrementInt` _pointeurx_2
          (:`  `
            (`/Engine/EditorBlueprintResources/StandardMacros.DecrementInt` _pointeury_4)))
        (else
          (set `self.IncreaseState` "NewEnumerator5")
          (`/Engine/EditorBlueprintResources/StandardMacros.DecrementInt` _pointeury_4 :!label _label_3
            (:`  `
              (if (`self.GetGridState` _pointeurx_2 _pointeury_4)
                (goto _label_3)))))))
    (:`NewEnumerator5`
      ;[1 1 1] Diag Bot Right
      (if (`self.GetGridState` (+ (`self.PointeurX`) -2) (+ (`self.PointeurY`) -1))
        (`/Engine/EditorBlueprintResources/StandardMacros.DecrementInt` _pointeury_5
          (:`  `
            (`/Engine/EditorBlueprintResources/StandardMacros.DecrementInt` _pointeurx_3)))
        (else
          (set `self.IncreaseState` "NewEnumerator6")
          (`/Engine/EditorBlueprintResources/StandardMacros.DecrementInt` _pointeurx_3 :!label _label_4
            (:`  `
              (if (`self.GetGridState` _pointeurx_3 _pointeury_5)
                (goto _label_4)))))))
    (:`NewEnumerator6`
      ;[1 1 1] Diag Bot Left
      (if (`self.GetGridState` (+ (`self.PointeurX`) -1) (+ (`self.PointeurY`) 2))
        (`/Engine/EditorBlueprintResources/StandardMacros.DecrementInt` _pointeurx
          (:`  `
            (`/Engine/EditorBlueprintResources/StandardMacros.IncrementInt` _pointeury_3)))
        (else
          (set `self.IncreaseState` "NewEnumerator7")
          (`/Engine/EditorBlueprintResources/StandardMacros.IncrementInt` _pointeury_3 :!label _label_5
            (:`  `
              (if (`self.GetGridState` _pointeurx _pointeury_3)
                (goto _label_5)))))))
    (:`NewEnumerator7`
      ;[1 1 1] Diag Top Left
      (if (`self.GetGridState` (+ (`self.PointeurX`) 2) (+ (`self.PointeurY`) 1))
        (`/Engine/EditorBlueprintResources/StandardMacros.IncrementInt` _pointeury_6
          (:`  `
            (`/Engine/EditorBlueprintResources/StandardMacros.IncrementInt` (`self.PointeurX`))))
        (else
          (set `self.IncreaseState` "NewEnumerator0")
          (`/Engine/EditorBlueprintResources/StandardMacros.IncrementInt` _pointeury_6))))))

(fn `Spawn Base City`
  (locals (Offset :type "Float (double-precision)" :default 1000.0) (BecomeBunker :type "/Game/BP/Building/BP_Habitation Object Reference"))
  (bind _offset (`local.Offset`))
  (bind _offset_2 (`local.Offset`))
  (bind _habitationlist (`self.HabitationList`))
  (for _index (range -3 4)
    (for _index_2 (range -3 4)
      (bind _returnvalue (== _index_2 -3))
      (bind _returnvalue_2 (== _index_2 3))
      (if (not (or (and (or (== _index -3) (== _index 3)) (or (== _index_2 -2) (== _index_2 2) _returnvalue _returnvalue_2)) (and (or (== _index -2) (== _index 2)) (or _returnvalue _returnvalue_2))))
        (bind _returnvalue_3 (`|SpawnActorFromClass` "/Game/BP/Building/BP_Habitation.BP_Habitation_C" (`KismetMathLibrary.MakeTransform` (`KismetMathLibrary.MakeVector` (* _offset _index) (* _offset _index_2) 100.0)) "Undefined" "OverrideRootScale" null _index _index_2 null))
        (`KismetArrayLibrary.Array_Set` (`self.GridData`) (`self.PosToIndex` _index _index_2) "NewEnumerator1")
        (`KismetArrayLibrary.Array_Add` (`self.HabitationList`) _returnvalue_3))))
  (bind _output_get (set `local.BecomeBunker` (`KismetArrayLibrary.Array_Random` _habitationlist)))
  (`KismetArrayLibrary.Array_RemoveItem` _habitationlist _output_get)
  (bind _gridx (`/Game/BP/Building/BP_BuildingParent.GridX` _output_get))
  (bind _gridy (`/Game/BP/Building/BP_BuildingParent.GridY` _output_get))
  (`|SpawnActorFromClass` "/Game/BP/Building/Bp_Bunker.Bp_Bunker_C" (`KismetMathLibrary.MakeTransform` (`KismetMathLibrary.MakeVector` (* _offset_2 _gridx) (* _offset_2 _gridy) 200.0)) "Undefined" "OverrideRootScale" null _gridx _gridy null)
  (`KismetArrayLibrary.Array_Set` (`self.GridData`) (`self.PosToIndex` _gridx _gridy) "NewEnumerator2")
  (`self.K2_DestroyActor` _output_get))

(fn `SpawnMeteor`
  (locals (Location :type "Array of Integer") (Offset :type "Float (double-precision)" :default 1000.0) (RdnInt :type Integer))
  (bind _location (`local.Location`))
  (bind _offset (`local.Offset`))
  (for (_array_element _array_index) (`self.GridData`)
    (if (`|EnumEquality` _array_element "NewEnumerator1")
      (`KismetArrayLibrary.Array_Add` (`local.Location`) _array_index)))
  (if (>= (`KismetArrayLibrary.Array_LastIndex` _location) 0)
    (bind _output_get (set `local.RdnInt` (`KismetArrayLibrary.Array_Random` _location)))
    (bind (_x _y) (`self.IndexToPos` _output_get))
    (`|SpawnActorFromClass` "/Game/BP/BP_Meteor.BP_Meteor_C" (`KismetMathLibrary.MakeTransform` (`KismetMathLibrary.MakeVector` (* _x _offset) (* _y _offset) 2000.0)) "Undefined" "OverrideRootScale" null null)
    (`KismetArrayLibrary.Array_Set` (`self.GridData`) _output_get "NewEnumerator3")
    (for _array_element_2 (`self.HabitationList`)
      (`/Engine/EditorBlueprintResources/StandardMacros.IsValid` _array_element_2
        (:`Is Valid`
          (if (and (== (`/Game/BP/Building/BP_BuildingParent.GridX` _array_element_2) _x) (== (`/Game/BP/Building/BP_BuildingParent.GridY` _array_element_2) _y))
            (`/Game/BP/Building/BP_Habitation.ActiveTarget` _array_element_2)
            (break)))))))

(fn `UserConstructionScript`)