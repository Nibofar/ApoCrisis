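; Bunker building that the player character can be offered to barricade.
; On BeginPlay it spawns a BP_CivilPos at the IsSanchezHere trigger's location and stores it as its Entry.
; Overlapping that trigger sets the third-person character's action button to Barricader only, not Evacuer, and registers the bunker as its current Building.
; Leaving the trigger hides the button.
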(event `self.ReceiveBeginPlay`
  (bind _returnvalue (`|SpawnActorFromClass` "/Game/BP/BP_CivilPos.BP_CivilPos_C" (`KismetMathLibrary.MakeTransform` (`SceneComponent.K2_GetComponentLocation` (`self.IsSanchezHere`))) "AlwaysSpawn" "OverrideRootScale" null null))
  (set `self.Entry` _returnvalue))

(event `self.IsSanchezHere.OnComponentBeginOverlap`
  (params (OverlappedComponent :type "PrimitiveComponent Object Reference") (OtherActor :type "Actor Object Reference") (OtherComp :type "PrimitiveComponent Object Reference") (OtherBodyIndex :type Integer) (bFromSweep :type Boolean) (SweepResult :type "HitResult Structure (by ref)"))
  (bind _asbp_third_person_character (cast `/Game/ThirdPerson/Blueprints/BP_ThirdPersonCharacter` OtherActor))
  (`/Game/ThirdPerson/Blueprints/BP_ThirdPersonCharacter.SetActifButton` _asbp_third_person_character false true)
  (set `/Game/ThirdPerson/Blueprints/BP_ThirdPersonCharacter.Building` self _asbp_third_person_character))

(event `self.IsSanchezHere.OnComponentEndOverlap`
  (params (OverlappedComponent :type "PrimitiveComponent Object Reference") (OtherActor :type "Actor Object Reference") (OtherComp :type "PrimitiveComponent Object Reference") (OtherBodyIndex :type Integer))
  (bind _asbp_third_person_character (cast `/Game/ThirdPerson/Blueprints/BP_ThirdPersonCharacter` OtherActor))
  (`/Game/ThirdPerson/Blueprints/BP_ThirdPersonCharacter.HideActifButton` _asbp_third_person_character))

(fn `UserConstructionScript`)