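; Residential building on the map grid that shelters civilians, offers the player evacuate or barricade actions, and can be destroyed by meteors.
; Construction randomizes storey count and civilians, then stacks visible floors.
; At BeginPlay the civilian count tints the shield effect; player overlap toggles action buttons by occupancy.
; Meteors hide upper floors; a ground-floor hit spawns BP_Ruin, updates BP_MapBehaviour's grid and calls End on a player in front.
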(event `self.ReceiveBeginPlay`
  (`self.SetColor`))

(event `self.IsSanchezHere.OnComponentBeginOverlap`
  (params (OverlappedComponent :type "PrimitiveComponent Object Reference") (OtherActor :type "Actor Object Reference") (OtherComp :type "PrimitiveComponent Object Reference") (OtherBodyIndex :type Integer) (bFromSweep :type Boolean) (SweepResult :type "HitResult Structure (by ref)"))
  (bind _civil (`self.Civil`))
  (bind _asbp_third_person_character (cast `/Game/ThirdPerson/Blueprints/BP_ThirdPersonCharacter` OtherActor))
  (bind _output_get (set `self.Character` _asbp_third_person_character))
  (set `/Game/ThirdPerson/Blueprints/BP_ThirdPersonCharacter.Building` self _output_get)
  (`/Game/ThirdPerson/Blueprints/BP_ThirdPersonCharacter.SetActifButton` _asbp_third_person_character (> _civil 0) (< _civil (* (`self.NbStairs`) 3)))
  (`/Game/ThirdPerson/Blueprints/BP_ThirdPersonCharacter.SetActifButton` _output_get (> _civil 0) (< _civil (* (`self.NbStairs`) 3)))
  (set `self.InFront` true))

(event `self.IsSanchezHere.OnComponentEndOverlap`
  (params (OverlappedComponent :type "PrimitiveComponent Object Reference") (OtherActor :type "Actor Object Reference") (OtherComp :type "PrimitiveComponent Object Reference") (OtherBodyIndex :type Integer))
  (bind _asbp_third_person_character (cast `/Game/ThirdPerson/Blueprints/BP_ThirdPersonCharacter` OtherActor))
  (`/Game/ThirdPerson/Blueprints/BP_ThirdPersonCharacter.HideActifButton` _asbp_third_person_character)
  (`KismetSystemLibrary.Delay` 0.2)
  (set `self.InFront` false))

(event `self.Roof.OnComponentBeginOverlap`
  (params (OverlappedComponent :type "PrimitiveComponent Object Reference") (OtherActor :type "Actor Object Reference") (OtherComp :type "PrimitiveComponent Object Reference") (OtherBodyIndex :type Integer) (bFromSweep :type Boolean) (SweepResult :type "HitResult Structure (by ref)"))
  (cast `/Game/BP/BP_Meteor` OtherActor)
  (`SceneComponent.SetVisibility` (`self.Roof`) false false))

(event `self.Floor 3.OnComponentBeginOverlap`
  (params (OverlappedComponent :type "PrimitiveComponent Object Reference") (OtherActor :type "Actor Object Reference") (OtherComp :type "PrimitiveComponent Object Reference") (OtherBodyIndex :type Integer) (bFromSweep :type Boolean) (SweepResult :type "HitResult Structure (by ref)"))
  (cast `/Game/BP/BP_Meteor` OtherActor)
  (`SceneComponent.SetVisibility` (`self.Floor 3`) false false))

(event `self.Floor 2.OnComponentBeginOverlap`
  (params (OverlappedComponent :type "PrimitiveComponent Object Reference") (OtherActor :type "Actor Object Reference") (OtherComp :type "PrimitiveComponent Object Reference") (OtherBodyIndex :type Integer) (bFromSweep :type Boolean) (SweepResult :type "HitResult Structure (by ref)"))
  (cast `/Game/BP/BP_Meteor` OtherActor)
  (`SceneComponent.SetVisibility` (`self.Floor 2`) false false))

(event `self.Floor 1.OnComponentBeginOverlap`
  (params (OverlappedComponent :type "PrimitiveComponent Object Reference") (OtherActor :type "Actor Object Reference") (OtherComp :type "PrimitiveComponent Object Reference") (OtherBodyIndex :type Integer) (bFromSweep :type Boolean) (SweepResult :type "HitResult Structure (by ref)"))
  (cast `/Game/BP/BP_Meteor` OtherActor)
  (`SceneComponent.SetVisibility` (`self.Floor 1`) false false))

(event `self.RDC.OnComponentBeginOverlap`
  (params (OverlappedComponent :type "PrimitiveComponent Object Reference") (OtherActor :type "Actor Object Reference") (OtherComp :type "PrimitiveComponent Object Reference") (OtherBodyIndex :type Integer) (bFromSweep :type Boolean) (SweepResult :type "HitResult Structure (by ref)"))
  (bind _gridx (`self.GridX`))
  (bind _gridy (`self.GridY`))
  (bind _asbp_meteor (cast `/Game/BP/BP_Meteor` OtherActor))
  (`self.K2_DestroyActor` _asbp_meteor)
  (bind _returnvalue (`GameplayStatics.GetActorOfClass` "/Game/BP/Building/BP_MapBehaviour.BP_MapBehaviour_C"))
  (`|SpawnActorFromClass` "/Game/BP/Building/BP_Ruin.BP_Ruin_C" (`KismetMathLibrary.MakeTransform` (`KismetMathLibrary.MakeVector` (* _gridx 1000.0) (* _gridy 1000.0) 25.0)) "Undefined" "OverrideRootScale" null 0 0 null)
  (bind _offsetgrid (`/Game/BP/Building/BP_MapBehaviour.OffsetGrid` _returnvalue))
  (bind _returnvalue_2 (/ _offsetgrid 2))
  (bind _returnvalue_3 (`KismetMathLibrary.Conv_IntToDouble` (* _returnvalue_2 -1)))
  (bind _returnvalue_4 (`KismetMathLibrary.Conv_IntToDouble` _returnvalue_2))
  (bind _returnvalue_5 (`KismetMathLibrary.Conv_IntToDouble` _offsetgrid))
  (`KismetArrayLibrary.Array_Set` (`/Game/BP/Building/BP_MapBehaviour.GridData` _returnvalue) (`KismetMathLibrary.FTrunc` (+ (* (`KismetMathLibrary.NormalizeToRange` (`KismetMathLibrary.Conv_IntToDouble` _gridx) _returnvalue_3 _returnvalue_4) _returnvalue_5 _returnvalue_5) (* (`KismetMathLibrary.NormalizeToRange` (`KismetMathLibrary.Conv_IntToDouble` _gridy) _returnvalue_3 _returnvalue_4) _returnvalue_5))) "NewEnumerator3")
  (if (`self.InFront`)
    (`/Game/ThirdPerson/Blueprints/BP_ThirdPersonCharacter.End` (`self.Character`)))
  (`self.K2_DestroyActor`))

(fn `SetColor`
  (bind _m_shieldeffect (`self.M_ShieldEffect`))
  (bind _returnvalue (- 1.0 (`KismetMathLibrary.NormalizeToRange` (`KismetMathLibrary.Conv_IntToDouble` (`self.Civil`)) 0.0 15.0)))
  (`FXSystemComponent.SetColorParameter` _m_shieldeffect "ShieldColor" (make `LinearColor` 0.0 _returnvalue 1.0 1.0))
  (`FXSystemComponent.SetColorParameter` _m_shieldeffect "CircleColor" (make `LinearColor` 0.0 _returnvalue 1.0 1.0)))

(fn `SetStairs`
  (bind _output_get (set `self.NbStairs` (`KismetMathLibrary.RandomIntegerInRange` 3 5)))
  (`|ExecutionSequence`
    (:`then_0`
      (switch `int` _output_get
        (:`3`
          (`SceneComponent.SetVisibility` (`self.Floor 3`) false false))
        (:`4`
          _))
      (`SceneComponent.SetVisibility` (`self.Floor 2`) false false))
    (:`then_1`
      (set `self.Civil` (`KismetMathLibrary.RandomIntegerInRange` _output_get (* _output_get 3))))))

(fn `SetVisibleStairs`
  (locals (Count :type Integer :default -1))
  (bind _count (`local.Count`))
  (for _array_element (`|MakeArray` (`self.RDC`) (`self.Floor 1`) (`self.Floor 2`) (`self.Floor 3`) (`self.Roof`))
    (if (`SceneComponent.IsVisible` _array_element)
      (`/Engine/EditorBlueprintResources/StandardMacros.IncrementInt` _count
        (:`  `
          (`SceneComponent.K2_SetRelativeLocation` _array_element (`KismetMathLibrary.MakeVector` 0.0 0.0 (* _count 200.0)) false false))))))

(fn `UserConstructionScript`
  (`parent.UserConstructionScript`)
  (`self.SetStairs`)
  (`self.SetVisibleStairs`))